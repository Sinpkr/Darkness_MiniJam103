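; Player controller for a card-battle game that runs the fight loop, player stats, deck and hand.
; BeginPlay resets stats from the boss data table, keeping any existing deck, then shows the enemy intro over a random cine camera.
; StartFight opens the HUD, and each turn deals five random cards from a fresh copy of the deck.
; NextFight fades out, saves the deck, advances the boss spawner and replays the intro.
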(event `Client_Pause`
  (`KismetSystemLibrary.PrintString` "Pause"))

(event `Set Stats`
  (bind _playerdetails (`self.PlayerDetails`))
  ;[0.07812 0 1] Resets Player
  (setmembers `/Game/AAA_DarkJam_103/Core/Characters/S_CharacterDetails` :`StructRef` _playerdetails)
  (if (not (`KismetArrayLibrary.Array_IsValidIndex` (`.CardDeck_27_0646244F46BEDF219F17939E5510AA52` (break `/Game/AAA_DarkJam_103/Core/Characters/S_CharacterDetails` _playerdetails)) 1))
    (bind _returnvalue (`|GetDataTableRow` "/Game/AAA_DarkJam_103/Characters/DT_BossDataTable.DT_BossDataTable" (`KismetStringLibrary.Conv_StringToName` (`KismetStringLibrary.Conv_IntToString` 10)))
      (:`then`
        (bind (_charid _name _charclasslevel _currenthealth _maxhealth _armour _effectmultiplyer _carddeck _image) (break `/Game/AAA_DarkJam_103/Core/Characters/S_CharacterDetails` _returnvalue))
        (setmembers `/Game/AAA_DarkJam_103/Core/Characters/S_CharacterDetails` :`StructRef` (`self.PlayerDetails`) :`CharID` _charid :`Name` _name :`CharClassLevel` _charclasslevel :`CurrentHealth` _currenthealth :`MaxHealth` _maxhealth :`Armour` _armour :`EffectMultiplyer` _effectmultiplyer :`CardDeck` _carddeck :`Image` _image)))
    (else
      (bind _returnvalue_2 (`|GetDataTableRow` "/Game/AAA_DarkJam_103/Characters/DT_BossDataTable.DT_BossDataTable" (`KismetStringLibrary.Conv_StringToName` (`KismetStringLibrary.Conv_IntToString` 10)))
        (:`then`
          (bind (_charid_2 _name_2 _charclasslevel_2 _currenthealth_2 _maxhealth_2 _armour_2 _effectmultiplyer_2 _carddeck_2 _image_2) (break `/Game/AAA_DarkJam_103/Core/Characters/S_CharacterDetails` _returnvalue_2))
          (setmembers `/Game/AAA_DarkJam_103/Core/Characters/S_CharacterDetails` :`StructRef` (`self.PlayerDetails`) :`CharID` _charid_2 :`Name` _name_2 :`CharClassLevel` _charclasslevel_2 :`CurrentHealth` _currenthealth_2 :`MaxHealth` _maxhealth_2 :`Armour` _armour_2 :`EffectMultiplyer` _effectmultiplyer_2 :`Image` _image_2))))))

(event `InputAction|Escape / Quit`
  (params (Key :type "Key Structure"))
  ;[0 0.8594 1] Comment
  (:`Pressed`
    (`KismetSystemLibrary.QuitGame` null "Quit")))

(event `self.ReceiveBeginPlay`
  (`self.Set Stats` :!label _label)
  (`PlayerCameraManager.StartCameraFade` :`self` (`GameplayStatics.GetPlayerCameraManager` 0) :`FromAlpha` 1.0 :`Duration` 1.0 :`bHoldWhenFinished` true)
  (`KismetSystemLibrary.Delay` 0.2)
  (bind _returnvalue (`|CreateWidget` "/Game/AAA_DarkJam_103/Core/UI/HUD/WBP_DarkEnemyIntro.WBP_DarkEnemyIntro_C"))
  (`UserWidget.AddToViewport` _returnvalue 0)
  (`WidgetBlueprintLibrary.SetInputMode_GameAndUIEx` self _returnvalue)
  (set `self.bShowMouseCursor` true)
  (bind _outactors (`GameplayStatics.GetAllActorsOfClass` "/Script/CinematicCamera.CineCameraActor"))
  (for _array_element _outactors
    (`KismetArrayLibrary.Array_Add` (`self.CameraArray`) _array_element))
  (`self.SetViewTargetWithBlend` (`KismetArrayLibrary.Array_Random` (`self.CameraArray`))))

(event `NextFight`
  (`PlayerCameraManager.StartCameraFade` :`self` (`GameplayStatics.GetPlayerCameraManager` 0) :`ToAlpha` 1.0 :`Duration` 2.0 :`bHoldWhenFinished` true)
  (setmembers `/Game/AAA_DarkJam_103/Core/Characters/S_CharacterDetails` :`StructRef` (`self.PlayerDetails`) :`CardDeck` (`self.TotalCards`))
  (`KismetSystemLibrary.Delay` 0.2)
  (`Widget.RemoveFromParent` (`self.PlayerHUD`))
  (`KismetArrayLibrary.Array_Clear` (`self.TotalCards`))
  (`KismetArrayLibrary.Array_Clear` (`self.CardsInHand`))
  (`KismetArrayLibrary.Array_Clear` (`self.CardsInGraveyard`))
  (bind _returnvalue (`GameplayStatics.GetActorOfClass` "/Game/AAA_DarkJam_103/Characters/BP_BossEnemySpawn.BP_BossEnemySpawn_C"))
  (`/Game/AAA_DarkJam_103/Characters/BP_BossEnemySpawn.NextFight` _returnvalue)
  (`KismetSystemLibrary.Delay` 2.0)
  (goto _label))

(event `StartFight`
  (`KismetSystemLibrary.Delay` 0.2)
  (bind _returnvalue (`|CreateWidget` "/Game/AAA_DarkJam_103/Core/UI/HUD/WBP_DarkPlayerHUD.WBP_DarkPlayerHUD_C"))
  (bind _output_get (set `self.PlayerHUD` _returnvalue))
  (`UserWidget.AddToViewport` _output_get 0)
  (`WidgetBlueprintLibrary.SetInputMode_GameAndUIEx` self _output_get)
  (set `self.bShowMouseCursor` true)
  (set `self.TotalCards` (`.CardDeck_27_0646244F46BEDF219F17939E5510AA52` (break `/Game/AAA_DarkJam_103/Core/Characters/S_CharacterDetails` (`self.PlayerDetails`))))
  (`self.FirstTurn`))

(event `FirstTurn`
  (bind _playerhud (`self.PlayerHUD`))
  (bind _returnvalue (+ (`self.Cards2Draw`) 1))
  (bind _returnvalue_2 (`KismetMathLibrary.RandomIntegerInRange` 0 (`KismetArrayLibrary.Array_LastIndex` (`self.DrawDeck`))))
  (set `self.DrawDeck` (`self.TotalCards`) :!label _label_2)
  (`KismetSystemLibrary.Delay` 0.2)
  (while (not (== (`self.Cards2Draw`) 5))
    (set `self.Cards2Draw` _returnvalue)
    (`KismetArrayLibrary.Array_Add` (`self.CardsInHand`) (`|GetArrayItem` (`self.DrawDeck`) _returnvalue_2))
    (`KismetArrayLibrary.Array_Remove` (`self.DrawDeck`) _returnvalue_2)
    (`KismetSystemLibrary.PrintString` (`KismetStringLibrary.Conv_IntToString` _returnvalue) false false))
  (set `self.Cards2Draw` 0)
  (set `/Game/AAA_DarkJam_103/Core/UI/HUD/WBP_DarkPlayerHUD.CardsInHand` (`self.CardsInHand`) _playerhud)
  (`/Game/AAA_DarkJam_103/Core/UI/HUD/WBP_DarkPlayerHUD.Refresh_Hand` _playerhud))

(event `PlayerTurn`
  (`KismetArrayLibrary.Array_Clear` (`self.CardsInHand`))
  (goto _label_2))

(fn `UserConstructionScript`)