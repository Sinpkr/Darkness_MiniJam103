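; BP_BossEnemySpawn picks the character details of the enemy for each fight, escalating as the fight round counter rises.
; BeginPlay loads a random row from the normal data table, and NextFight advances the round, switching to a random boss-table row at round three.
; From round four, boss row 10 is overwritten with the player controller's identity, card deck and image plus boosted stats, creating a mirror-match boss.
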(event `self.ReceiveBeginPlay`
  (bind _returnvalue (`|GetDataTableRow` "/Game/AAA_DarkJam_103/Characters/DT_NormalDataTable.DT_NormalDataTable" (`KismetStringLibrary.Conv_StringToName` (`KismetStringLibrary.Conv_IntToString` (`KismetMathLibrary.RandomIntegerInRange` 1 (`self.TotalBosses`)))))
    (:`then`
      (bind _output_get (set `self.CharcterDetails` _returnvalue))
      (set `self.Char ID` (`.CharID_13_3D29C37841DF0130CF3412A4921FE1D9` (break `/Game/AAA_DarkJam_103/Core/Characters/S_CharacterDetails` _output_get)))
      (set `self.FightRound` (+ (`self.FightRound`) 1)))))

(event `NextFight`
  (set `self.FightRound` (+ (`self.FightRound`) 1))
  (if (< (`self.FightRound`) 3)
    (bind _returnvalue (`|GetDataTableRow` "/Game/AAA_DarkJam_103/Characters/DT_NormalDataTable.DT_NormalDataTable" (`KismetStringLibrary.Conv_StringToName` (`KismetStringLibrary.Conv_IntToString` (`KismetMathLibrary.RandomIntegerInRange` 1 (`self.TotalBosses`)))))
      (:`then`
        (bind _output_get (set `self.CharcterDetails` _returnvalue))
        (set `self.Char ID` (`.CharID_13_3D29C37841DF0130CF3412A4921FE1D9` (break `/Game/AAA_DarkJam_103/Core/Characters/S_CharacterDetails` _output_get)))))
    (elif (< (`self.FightRound`) 4)
      (bind _returnvalue_2 (`|GetDataTableRow` "/Game/AAA_DarkJam_103/Characters/DT_BossDataTable.DT_BossDataTable" (`KismetStringLibrary.Conv_StringToName` (`KismetStringLibrary.Conv_IntToString` (`KismetMathLibrary.RandomIntegerInRange` 1 (`self.TotalBosses`)))))
        (:`then`
          (bind _output_get_2 (set `self.CharcterDetails` _returnvalue_2))
          (set `self.Char ID` (`.CharID_13_3D29C37841DF0130CF3412A4921FE1D9` (break `/Game/AAA_DarkJam_103/Core/Characters/S_CharacterDetails` _output_get_2)))))
      (else
        (bind _returnvalue_3 (`|GetDataTableRow` "/Game/AAA_DarkJam_103/Characters/DT_BossDataTable.DT_BossDataTable" (`KismetStringLibrary.Conv_StringToName` (`KismetStringLibrary.Conv_IntToString` 10)))
          (:`then`
            (set `self.CharcterDetails` _returnvalue_3)
            (bind _asbp_dark_player_controller (cast `/Game/AAA_DarkJam_103/Core/Player/BP_DarkPlayerController` (`GameplayStatics.GetPlayerController` 0)))
            (bind (_charid _name _charclasslevel _currenthealth _maxhealth _armour _effectmultiplyer _carddeck _image) (break `/Game/AAA_DarkJam_103/Core/Characters/S_CharacterDetails` (`/Game/AAA_DarkJam_103/Core/Player/BP_DarkPlayerController.PlayerDetails` _asbp_dark_player_controller)))
            (bind _returnvalue_4 (+ _maxhealth 20.0))
            (bind _structout (setmembers `/Game/AAA_DarkJam_103/Core/Characters/S_CharacterDetails` :`StructRef` (`self.CharcterDetails`) :`CharID` _charid :`Name` _name :`CharClassLevel` _charclasslevel :`CurrentHealth` _returnvalue_4 :`MaxHealth` _returnvalue_4 :`Armour` 5.0 :`EffectMultiplyer` 2.0 :`CardDeck` _carddeck :`Image` _image))
            (set `self.Char ID` (`.CharID_13_3D29C37841DF0130CF3412A4921FE1D9` (break `/Game/AAA_DarkJam_103/Core/Characters/S_CharacterDetails` _structout)))))))))

(fn `UserConstructionScript`
  (`parent.UserConstructionScript`))